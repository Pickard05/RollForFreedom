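; BP_Dice is a physics-driven six-sided die that throws itself on BeginPlay and prints the face that lands up.
; The roll enables physics on SMDice and applies an impulse along the player character's forward vector.
; After a delay, it repeatedly compares actor locations over short intervals until the die stops moving.
; GetDiceResult then picks the first face component whose forward vector roughly matches world up and prints its name.
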(event Custom|roll%20Dice
  (bind _sm_dice (Variables|Default|GetSM_Dice))
  (Physics|SetSimulatePhysics _sm_dice true)
  (Physics|AddImpulse _sm_dice (* (Transformation|GetActorForwardVector (Game|GetPlayerCharacter 0)) 2.5e+02) "None" true)
  (Utilities|FlowControl|Delay 2.0)
  (CallFunction|StoppedRolling?))

(event Custom|Stopped%20rolling?
  (bind _returnvalue (Transformation|GetActorLocation))
  (Variables|Default|SetStopped%20Location _returnvalue)
  (Utilities|FlowControl|Delay 0.5)
  (if (Utilities|Operators|EqualEqual (Variables|Default|GetStopped%20Location) _returnvalue 1e-05)
    (CallFunction|GetDiceResult)
    (else
      (CallFunction|StoppedRolling?))))

(event EventBeginPlay
  (CallFunction|RollDice))

(event Collision|EventActorBeginOverlap
  (params (OtherActor :type Actor%20Object%20Reference)))

(event EventTick
  (params (DeltaSeconds :type Float%20%28single-precision%29)))

(fn ConstructionScript)

(fn GetDiceResult
  (if (Utilities|Operators|EqualEqual (Math|Vector|GetForwardVector (Variables|Default|GetFace%201)) "0.000000,0.000000,1.000000" 0.5)
    (Variables|Default|SetResulted%20Face (Variables|Default|GetFace%201))
    (Development|PrintString (Utilities|GetDisplayName (Variables|Default|GetResulted%20Face)) :!label _label)
    (return)
    (elif (Utilities|Operators|EqualEqual (Math|Vector|GetForwardVector (Variables|Default|GetFace%202)) "0.000000,0.000000,1.000000" 0.5)
      (Variables|Default|SetResulted%20Face (Variables|Default|GetFace%202))
      (goto _label)
      (elif (Utilities|Operators|EqualEqual (Math|Vector|GetForwardVector (Variables|Default|GetFace%203)) "0.000000,0.000000,1.000000" 0.5)
        (Variables|Default|SetResulted%20Face (Variables|Default|GetFace%203))
        (goto _label)
        (elif (Utilities|Operators|EqualEqual (Math|Vector|GetForwardVector (Variables|Default|GetFace%204)) "0.000000,0.000000,1.000000" 0.5)
          (Variables|Default|SetResulted%20Face (Variables|Default|GetFace%204))
          (goto _label)
          (elif (Utilities|Operators|EqualEqual (Math|Vector|GetForwardVector (Variables|Default|GetFace%205)) "0.000000,0.000000,1.000000" 0.5)
            (Variables|Default|SetResulted%20Face (Variables|Default|GetFace%205))
            (goto _label)
            (elif (Utilities|Operators|EqualEqual (Math|Vector|GetForwardVector (Variables|Default|GetFace%206)) "0.000000,0.000000,1.000000" 0.5)
              (Variables|Default|SetResulted%20Face (Variables|Default|GetFace%206))
              (goto _label))))))))