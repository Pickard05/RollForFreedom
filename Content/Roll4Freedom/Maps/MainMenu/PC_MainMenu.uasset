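; PC_MainMenu is the player controller for the Roll4Freedom main menu, handling the interaction UI and seated look limits.
; On BeginPlay, the local controller creates the WB_InteractWidget once and adds it to the viewport.
; While SatDown is true, Tick clamps camera manager yaw to an arc centered on the controlled pawn's root facing, and prints a leftover-looking debug string every frame.
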(event EventBeginPlay
  (if (Pawn|IsLocalPlayerController)
    (Utilities|FlowControl|DoOnce false
      (:Completed
        (bind _returnvalue (UserInterface|CreateWidget "/Game/UI/WB_InteractWidget.WB_InteractWidget_C" self))
        (UserInterface|Viewport|AddtoViewport _returnvalue 0)))))

(event EventTick
  (params (DeltaSeconds :type Float%20%28single-precision%29))
  (bind _returnvalue (Game|GetPlayerCameraManager 0))
  (bind _returnvalue_2 (Pawn|GetControlledPawn))
  (bind _rootcomponent (Variables|/Script/Engine.Actor|GetRootComponent _returnvalue_2))
  (bind _returnvalue_3 (Transformation|GetWorldRotation _rootcomponent))
  (if (Variables|Default|GetSatDown?)
    (Variables|/Script/Engine.PlayerCameraManager|SetViewYawMin _returnvalue (+ (.yaw _returnvalue_3) -7e+01))
    (Variables|/Script/Engine.PlayerCameraManager|SetViewYawMax _returnvalue (+ (.yaw _returnvalue_3) 7e+01))
    (Development|PrintString "Hello")))

(fn ConstructionScript)