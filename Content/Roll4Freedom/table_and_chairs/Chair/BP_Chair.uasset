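; BP_Chair is a chair actor in Roll4Freedom that tracks whether it is occupied.
; When the player's controlled pawn overlaps its Box, it prints a prompt to sit down, or to sit elsewhere if Occupied is set.
; Interact sets Occupied and returns false; this file contains no seating movement and nothing that clears the flag.
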(event OnComponentBeginOverlap(Box)
  (params (OverlappedComponent :type Primitive%20Component%20Object%20Reference) (OtherActor :type Actor%20Object%20Reference) (OtherComp :type Primitive%20Component%20Object%20Reference) (OtherBodyIndex :type Integer) (bFromSweep :type Boolean) (SweepResult :type Hit%20Result%20Structure%20%28by%20ref%29))
  (if (== OtherActor (Pawn|GetControlledPawn (Game|GetPlayerController 0)))
    (if (Variables|Default|GetOccupied)
      (Development|PrintString "Sit somewhere else PUNK.")
      (else
        (Development|PrintString "Sit down.")))))

(event EventBeginPlay)

(event Collision|EventActorBeginOverlap
  (params (OtherActor :type Actor%20Object%20Reference)))

(event EventTick
  (params (DeltaSeconds :type Float%20%28single-precision%29)))

(fn ConstructionScript)

(fn Interact
  (params (Interactor :type Actor%20Object%20Reference))
  (Variables|Default|SetOccupied true)
  (return false))