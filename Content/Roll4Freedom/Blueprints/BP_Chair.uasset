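; BP_Chair is an interactable chair whose prompt reads "Sit Down" while free and "Find Another Chair" once occupied.
; Interact calls SR_OccupySeat on both branches of ServerInteract, which passes through RPC_OccupySeat to set the Occupied flag.
; Interact never checks that flag, and nothing here clears it or moves the player into the seat.
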(event Custom|SR_OccupySeat
  (CallFunction|RPCOccupySeat))

(event Custom|RPC_OccupySeat
  (Variables|Default|SetOccupied true))

(event EventBeginPlay)

(event Collision|EventActorBeginOverlap
  (params (OtherActor :type Actor%20Object%20Reference)))

(event EventTick
  (params (DeltaSeconds :type Float%20%28single-precision%29)))

(event EventInteract
  (params (Interactor :type Actor%20Object%20Reference) (ServerInteract? :type Boolean))
  (if ServerInteract?
    (CallFunction|SROccupySeat)
    (else
      (CallFunction|SROccupySeat))))

(fn ConstructionScript)

(fn GetInteractData
  (if (Variables|Default|GetOccupied)
    (return "Find Another Chair")
    (else
      (return "Sit Down"))))