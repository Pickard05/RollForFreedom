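; Cell door Blueprint that swings open and closed when interacted with.
; Interact, gated by its ServerInteract flag, calls a server RPC event that relays to a second RPC event driving the door.
; That event uses a FlipFlop to alternately play the OpenClose timeline forward and in reverse, lerping the Door component's relative rotation through 85 degrees.
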(event Custom|RPC%20Open/Close%20Door
  ;[0.15 0.15 0.15 0.5] RPC/SR Open Close Door
  (Utilities|FlowControl|FlipFlop
    (:A
      (bind _rotate (Timeline|OpenClose PlayFromStart)
        (:Update
          (Transformation|SetRelativeRotation (Variables|Default|GetDoor) (Math|Rotator|Lerp(Rotator) "0, 0, 0" "0.0,-85.000000,0.0" _rotate true) false false))))
    (:B
      (Timeline|OpenClose ReverseFromEnd))))

(event Custom|SR_RPC%20Open/Close
  ;[0.15 0.15 0.15 0.5] RPC/SR Open Close Door
  (CallFunction|RPCOpen/CloseDoor))

(event EventInteract
  (params (Interactor :type Actor%20Object%20Reference) (ServerInteract? :type Boolean))
  ;[0.15 0.15 0.15 0.5] RPC/SR Open Close Door
  (if ServerInteract?
    (CallFunction|SRRPCOpen/Close)))

(fn ConstructionScript
  (|CallParentFunction))