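; BP_ChairNew is an interactable chair that players can sit on, with a prompt reading "Sit Down" or "Occupied".
; Interact calls SR_OccupySeat on either branch, which forwards to RPC_OccupySeat to set Occupied; nothing here clears it.
; SceneLocationInfo, also run on BeginPlay, records and returns the sit-down scene's world transform (location and rotation) and the stationary sit point's location.
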(event Custom|SR_OccupySeat
  (CallFunction|RPCOccupySeat))

(event Custom|RPC_OccupySeat
  (Variables|Default|SetOccupied true))

(event EventBeginPlay
  (|CallParentFunction)
  (CallFunction|SceneLocationInfo))

(event Collision|EventActorBeginOverlap
  (params (OtherActor :type Actor%20Object%20Reference))
  (|CallParentFunction OtherActor) ; This node is disabled and will not be called.\nDrag off pins to build functionality.
)

(event EventTick
  (params (DeltaSeconds :type Float%20%28single-precision%29))
  (|CallParentFunction DeltaSeconds) ; This node is disabled and will not be called.\nDrag off pins to build functionality.
)

(event EventInteract
  (params (Interactor :type Actor%20Object%20Reference) (ServerInteract? :type Boolean))
  (if ServerInteract?
    (CallFunction|SROccupySeat)
    (else
      (CallFunction|SROccupySeat))))

(fn ConstructionScript
  (|CallParentFunction))

(fn GetInteractData
  (if (Variables|Default|GetOccupied)
    (return "Occupied")
    (else
      (return "Sit Down"))))

(fn SceneLocationInfo
  (bind _sitdownscene (Variables|Default|GetSitDownScene))
  (bind _output_get (Variables|Default|SetSceneWorldRotation (Transformation|GetWorldRotation _sitdownscene)))
  (bind _output_get_2 (Variables|Default|SetSceneWorldLocation (Transformation|GetWorldLocation _sitdownscene)))
  (bind _output_get_3 (Variables|Default|SetChairWorldLocation (Transformation|GetWorldLocation (Variables|Default|GetStationarySitScene))))
  (return _output_get_2 _output_get _output_get_3))